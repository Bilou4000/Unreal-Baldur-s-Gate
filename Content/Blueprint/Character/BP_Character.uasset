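; BP_Character is a character Blueprint that tracks the coins and health of its character.
; On BeginPlay it copies both starting values from BdtStats.
; GetItem checks the item's actor tag: a good coin adds one coin, while a bad coin subtracts a random amount up to the stats' maximum loss.
; TakeDamage and Heal adjust health without clamping and print the result to screen.
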(event EventBeginPlay
  ;[1 1 1] Begin Play
  (Variables|stats|Setcoins (Variables|/Game/Blueprint/BDA/BDT_Stats.BDT_Stats_C|Getcoins (Variables|BDT|GetbdtStats)))
  (Variables|stats|Sethealth (Variables|/Game/Blueprint/BDA/BDT_Stats.BDT_Stats_C|Gethealth (Variables|BDT|GetbdtStats))))

(event EventTakeDamage
  (params (damage :type Float%20%28double-precision%29))
  ;[1 1 1] Take Damage
  (bind _output_get (Variables|stats|Sethealth (- (Variables|stats|Gethealth) damage)))
  (Development|PrintString (Utilities|String|ToString(Float) _output_get)))

(event EventHeal
  (params (healAmount :type Float%20%28double-precision%29))
  ;[1 1 1] Heal
  (bind _output_get (Variables|stats|Sethealth (+ (Variables|stats|Gethealth) healAmount)))
  (Development|PrintString (Utilities|String|ToString(Float) _output_get)))

(event EventGetItem
  (params (item :type Actor%20Object%20Reference))
  ;[1 1 1] Get item
  ;;[1 0.6355 0.1939] GoodCoin
  (if (Actor|ActorHasTag item "goodCoin")
    (Variables|stats|Setcoins (+ (Variables|stats|Getcoins) 1))
    (else
      ;;[1 0.2448 0.1851] BadCoin
      (if (Actor|ActorHasTag item "badCoin")
        (Variables|stats|Setcoins (- (Variables|stats|Getcoins) (Math|Random|RandomIntegerinRange 0 (Variables|/Game/Blueprint/BDA/BDT_Stats.BDT_Stats_C|GetmaxCoinsToLose (Variables|BDT|GetbdtStats)))))))))

(fn ConstructionScript)