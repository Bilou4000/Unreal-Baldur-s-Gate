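; BP_Camera is a camera Blueprint that smooths zoom through its spring arm's length.
; On BeginPlay it stores the arm's starting length as the desired length.
; Each tick it lerps the current length toward that target, with delta time times Btd's ZoomSmoothSpeed as alpha.
; Nothing in this file changes the desired length after initialization.
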(event EventBeginPlay
  ;[1 1 1] Begin Play
  (Variables|Default|SetDesireArmLenght (Variables|/Script/Engine.SpringArmComponent|GetTargetArmLength (Variables|Default|GetSpringArm))))

(event EventTick
  (params (DeltaSeconds :type Float%20%28single-precision%29))
  ;[1 1 1] Update
  (Variables|/Script/Engine.SpringArmComponent|SetTargetArmLength (Variables|Default|GetSpringArm) (Math|Float|Lerp (Variables|/Script/Engine.SpringArmComponent|GetTargetArmLength (Variables|Default|GetSpringArm)) (Variables|Default|GetDesireArmLenght) (* DeltaSeconds (Variables|/Game/Blueprint/BDA/BDT_Camera.BDT_Camera_C|GetzoomSmoothSpeed (Variables|Default|Getbtd))))))

(fn ConstructionScript)