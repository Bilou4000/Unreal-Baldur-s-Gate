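; BP_InfernalMetal is an Infernal Iron pickup actor that spins and bobs in place until collected.
; Tick applies frame-rate-scaled yaw to the actor and moves Body on a sine wave around its starting relative height.
; Interact prints collection and healing messages and destroys the actor, with no actual healing logic.
; Capsule overlap with a component tagged "character" also destroys it, silently.
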(event OnComponentBeginOverlap(Capsule)
  (params (OverlappedComponent :type Primitive%20Component%20Object%20Reference) (OtherActor :type Actor%20Object%20Reference) (OtherComp :type Primitive%20Component%20Object%20Reference) (OtherBodyIndex :type Integer) (bFromSweep :type Boolean) (SweepResult :type Hit%20Result%20Structure%20%28by%20ref%29))
  ;[1 1 1] Check if Overlap
  (if (Components|ComponentHasTag OtherComp "character")
    (Actor|DestroyActor)))

(event EventInteract
  ;[1 1 1] Interact On Click
  (Development|PrintString "Infernal Iron Collected!")
  (Actor|DestroyActor)
  (Development|PrintString "You have healed!"))

(event EventTick
  (params (DeltaSeconds :type Float%20%28single-precision%29))
  ;[1 1 1] Rotate Object
  (Transformation|AddActorLocalRotation (Math|Rotator|MakeRotator 0.0 0.0 (* DeltaSeconds (Variables|Default|GetYawPersecond))) false false)
  (Transformation|SetRelativeLocation (Variables|Default|GetBody) (Math|Vector|MakeVector 0.0 0.0 (+ (Variables|Default|GetRelativeStartingLocationZ) (* (Math|Trig|Sin(Degrees) (* (Actor|GetGameTimeSinceCreation) (Variables|Default|GetBobbing%20Speed))) (Variables|Default|GetBobbin%20Distance)))) false false))

(event EventBeginPlay
  ;[1 1 1] Begin Play
  (Variables|Default|SetRelativeStartingLocationZ (.z (.location (Transformation|GetRelativeTransform (Variables|Default|GetBody))))))

(fn ConstructionScript)