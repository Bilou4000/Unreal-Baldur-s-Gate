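; BP_FalseCoin is an interactive decoy coin pickup that tells the player they lost some coins.
; When a component tagged "character" overlaps Sphere1, it sends GetItemMessage with itself to that actor, prints the message and destroys itself after a short delay.
; An Interact event prints the same message and destroys the coin sooner, without notifying any actor.
; The coin itself changes no coin count.
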(event OnComponentBeginOverlap(Sphere1)
  (params (OverlappedComponent :type Primitive%20Component%20Object%20Reference) (OtherActor :type Actor%20Object%20Reference) (OtherComp :type Primitive%20Component%20Object%20Reference) (OtherBodyIndex :type Integer) (bFromSweep :type Boolean) (SweepResult :type Hit%20Result%20Structure%20%28by%20ref%29))
  ;[1 1 1] Get coin
  (if (Components|ComponentHasTag OtherComp "character")
    (Class|BPICharacter|GetItem(Message) OtherActor self)
    (Development|PrintString "You lost some coins...")
    (Utilities|FlowControl|Delay 1.0)
    (Actor|DestroyActor)))

(event EventInteract
  ;[1 1 1] Get coin
  (Development|PrintString "You lost some coins...")
  (Utilities|FlowControl|Delay 0.1)
  (Actor|DestroyActor))

(fn ConstructionScript)