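; Player controller for a point-and-click game that drives a free camera pawn (BP_Camera) and a separate BP_Character.
; Enhanced Input actions pan the camera, set its clamped zoom target and rotate the spring arm with mouse delta, tuned by BdtActions values.
; Clicks trace from the cursor, calling InteractMessage on "interactive"-tagged hits or otherwise sliding the character to the hit point with MoveComponentTo, without pathfinding.
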(event Input|EnhancedActionEvents|EnhancedInputActionIA_GyroscopeCamera
  (params (ActionValue :type Boolean) (ElapsedSeconds :type Float%20%28double-precision%29) (TriggeredSeconds :type Float%20%28double-precision%29) (InputAction :type Input%20Action%20Object%20Reference :default "/Game/Input/IA_GyroscopeCamera.IA_GyroscopeCamera"))
  (bind _as_bp_camera (Variables|Default|GetAs%20BP%20Camera))
  (bind _as_bp_camera_2 (Variables|Default|GetAs%20BP%20Camera))
  (bind _springarm (Variables|/Game/Blueprint/BP_Camera.BP_Camera_C|GetSpringArm _as_bp_camera))
  (bind _springarm_2 (Variables|/Game/Blueprint/BP_Camera.BP_Camera_C|GetSpringArm _as_bp_camera_2))
  (bind _returnvalue (Transformation|GetWorldRotation _springarm))
  (bind _returnvalue_2 (Transformation|GetWorldRotation _springarm_2))
  ;[1 1 1] Gyroscope Camera
  (Transformation|SetWorldRotation (Variables|/Game/Blueprint/BP_Camera.BP_Camera_C|GetSpringArm (Variables|Default|GetAs%20BP%20Camera)) (Math|Rotator|MakeRotator (.roll _returnvalue_2) (.pitch _returnvalue_2) (+ (.yaw _returnvalue_2) (* (.DeltaX (Class|PlayerController|GetInputMouseDelta)) (Variables|/Game/DataAsset/BDT_Actions.BDT_Actions_C|GetspeedGyroscope (Variables|Default|GetbdtActions))))) false false)
  (Transformation|SetWorldRotation (Variables|/Game/Blueprint/BP_Camera.BP_Camera_C|GetSpringArm (Variables|Default|GetAs%20BP%20Camera)) (Math|Rotator|MakeRotator (.roll _returnvalue) (+ (.pitch _returnvalue) (* (.DeltaY (Class|PlayerController|GetInputMouseDelta)) (Variables|/Game/DataAsset/BDT_Actions.BDT_Actions_C|GetspeedGyroscope (Variables|Default|GetbdtActions)))) (.yaw _returnvalue)) false false))

(event Input|EnhancedActionEvents|EnhancedInputActionIA_MoveCamera
  (params (ActionValue :type Vector%202D%20Structure) (ElapsedSeconds :type Float%20%28double-precision%29) (TriggeredSeconds :type Float%20%28double-precision%29) (InputAction :type Input%20Action%20Object%20Reference :default "/Game/Input/IA_MoveCamera.IA_MoveCamera"))
  (bind _as_bp_camera (Variables|Default|GetAs%20BP%20Camera))
  (bind _as_bp_camera_2 (Variables|Default|GetAs%20BP%20Camera))
  ;[1 1 1] Camera Move
  (Pawn|Input|AddMovementInput _as_bp_camera_2 (Math|Vector|GetRightVector (Variables|/Game/Blueprint/BP_Camera.BP_Camera_C|GetCamera _as_bp_camera_2)) (* (.x ActionValue) (Variables|/Game/DataAsset/BDT_Actions.BDT_Actions_C|GetsideSpeed (Variables|Default|GetbdtActions))) false)
  (Pawn|Input|AddMovementInput _as_bp_camera (Math|Vector|GetForwardVector (Variables|/Game/Blueprint/BP_Camera.BP_Camera_C|GetCamera _as_bp_camera)) (* (.y ActionValue) (Variables|/Game/DataAsset/BDT_Actions.BDT_Actions_C|GetforwardSpeed (Variables|Default|GetbdtActions))) false))

(event Input|EnhancedActionEvents|EnhancedInputActionIA_Zoom
  (params (ActionValue :type Float%20%28double-precision%29) (ElapsedSeconds :type Float%20%28double-precision%29) (TriggeredSeconds :type Float%20%28double-precision%29) (InputAction :type Input%20Action%20Object%20Reference :default "/Game/Input/IA_Zoom.IA_Zoom"))
  (bind _bdtactions (Variables|Default|GetbdtActions))
  ;[1 1 1] Camera Zoom
  (Variables|/Game/Blueprint/BP_Camera.BP_Camera_C|SetDesireArmLenght (Variables|Default|GetAs%20BP%20Camera) (Math|Float|Clamp(Float) (+ (Variables|/Game/Blueprint/BP_Camera.BP_Camera_C|GetDesireArmLenght (Variables|Default|GetAs%20BP%20Camera)) (* (* ActionValue -1.0) (Variables|/Game/DataAsset/BDT_Actions.BDT_Actions_C|GetzoomInputStep (Variables|Default|GetbdtActions)))) (Variables|/Game/DataAsset/BDT_Actions.BDT_Actions_C|GetminZoom _bdtactions) (Variables|/Game/DataAsset/BDT_Actions.BDT_Actions_C|GetmaxZoom _bdtactions))))

(event Input|EnhancedActionEvents|EnhancedInputActionIA_Move
  (params (ActionValue :type Boolean) (ElapsedSeconds :type Float%20%28double-precision%29) (TriggeredSeconds :type Float%20%28double-precision%29) (InputAction :type Input%20Action%20Object%20Reference :default "/Game/Input/IA_Move.IA_Move"))
  (bind (_worldlocation _worlddirection) (Game|Player|ConvertMouseLocationToWorldSpace))
  ;[1 1 1] IA move on click
  (:Started
    (bind _outhit (Collision|LineTraceByChannel _worldlocation (+ _worldlocation (* _worlddirection 5e+03)) "TraceTypeQuery1" false (Variables|Default|GetActors%20to%20Ignore) "ForDuration"))
    (if (not (Components|ComponentHasTag (.hitcomponent _outhit) "interactive"))
      (bind _output_get (Variables|Default|SetnewLocation (.location _outhit)))
      (Components|MoveComponentTo (Variables|/Script/Engine.Actor|GetRootComponent (Variables|Default|GetAICharacter)) _output_get "0, 0, 0" false false (Variables|/Game/DataAsset/BDT_Actions.BDT_Actions_C|GetmoveSpeed (Variables|Default|GetbdtActions)) false)
      (else
        (Class|BPIInteraction|Interact(Message) (.hitactor _outhit))))))

(event EventBeginPlay
  (bind _returnvalue (PlayerController|LocalPlayerSubsystems|GetEnhancedInputLocalPlayerSubsystem))
  (bind _actors_to_ignore (Variables|Default|GetActors%20to%20Ignore))
  ;[1 1 1] Begin Play
  (bind _asbp_camera (Utilities|Casting|CastToBP_Camera (Game|Player|GetPlayerPawn 0)))
  (Variables|Default|SetAs%20BP%20Camera _asbp_camera)
  (Utilities|IsValid _returnvalue
    (:Is%20Valid
      (Input|AddMappingContext _returnvalue "/Game/Input/IC_Character.IC_Character" 0 "(bIgnoreAllPressedKeysUntilRelease=True,bForceImmediately=False,bNotifyUserSettings=False)")
      (Variables|Default|SetbShowMouseCursor true)
      (bind _returnvalue_2 (Actor|GetActorOfClass "/Game/Blueprint/BP_Character.BP_Character_C"))
      (Variables|Default|SetAICharacter _returnvalue_2)
      (Utilities|Array|Add _actors_to_ignore (Variables|Default|GetAICharacter))
      (Utilities|Array|Add _actors_to_ignore (Variables|Default|GetAs%20BP%20Camera)))))

(fn ConstructionScript)

(fn GetWorldLocation
  (params (location :type Vector :default "0, 0, 0"))
  (return false))