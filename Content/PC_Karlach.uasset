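; PC_Karlach is a player controller that drives a BP_Camera pawn with Enhanced Input.
; On BeginPlay it caches the pawn and adds the IC_Character mapping context.
; IA_MoveCamera moves the pawn along the capsule's right vector and the camera's forward vector, with separate side and forward speeds.
; IA_Zoom changes the spring arm length by the inverted input scaled by ZoomSpeed, with no clamping.
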(event Input|EnhancedActionEvents|EnhancedInputActionIA_MoveCamera
  (params (ActionValue :type Vector%202D%20Structure) (ElapsedSeconds :type Float%20%28double-precision%29) (TriggeredSeconds :type Float%20%28double-precision%29) (InputAction :type Input%20Action%20Object%20Reference :default "/Game/Input/IA_MoveCamera.IA_MoveCamera"))
  (bind _as_bp_camera (Variables|Default|GetAs%20BP%20Camera))
  (bind _as_bp_camera_2 (Variables|Default|GetAs%20BP%20Camera))
  (:Triggered
    (Pawn|Input|AddMovementInput _as_bp_camera_2 (Math|Vector|GetRightVector (Variables|/Script/Engine.Character|GetCapsuleComponent _as_bp_camera_2)) (* (.x ActionValue) (Variables|Default|GetsideSpeed)) false)
    (Pawn|Input|AddMovementInput _as_bp_camera (Math|Vector|GetForwardVector (Variables|/Game/Blueprint/BP_Camera.BP_Camera_C|GetCamera _as_bp_camera)) (* (.y ActionValue) (Variables|Default|GetforwardSpeed)) false)))

(event Input|EnhancedActionEvents|EnhancedInputActionIA_Zoom
  (params (ActionValue :type Float%20%28double-precision%29) (ElapsedSeconds :type Float%20%28double-precision%29) (TriggeredSeconds :type Float%20%28double-precision%29) (InputAction :type Input%20Action%20Object%20Reference :default "/Game/Input/IA_Zoom.IA_Zoom"))
  (bind _as_bp_camera (Variables|Default|GetAs%20BP%20Camera))
  (bind _springarm (Variables|/Game/Blueprint/BP_Camera.BP_Camera_C|GetSpringArm _as_bp_camera))
  (:Triggered
    (Variables|/Script/Engine.SpringArmComponent|SetTargetArmLength _springarm (+ (Variables|/Script/Engine.SpringArmComponent|GetTargetArmLength _springarm) (* (* ActionValue -1.0) (Variables|Default|GetzoomSpeed))))))

(event EventBeginPlay
  (bind _returnvalue (PlayerController|LocalPlayerSubsystems|GetEnhancedInputLocalPlayerSubsystem))
  (bind _asbp_camera (Utilities|Casting|CastToBP_Camera (Game|Player|GetPlayerPawn 0)))
  (Variables|Default|SetAs%20BP%20Camera _asbp_camera)
  (Utilities|IsValid _returnvalue
    (:Is%20Valid
      (Input|AddMappingContext _returnvalue "/Game/Input/IC_Character.IC_Character" 0 "(bIgnoreAllPressedKeysUntilRelease=True,bForceImmediately=False,bNotifyUserSettings=False)"))))

(fn ConstructionScript)