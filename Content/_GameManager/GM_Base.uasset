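; GM_Base is a base game mode that sets up the game's save when play begins and can reload it through a LoadGame event.
; It loads a BP_GameSave from a fixed slot and passes it to the GI_Base game instance for use across levels.
; If no save exists, it creates and writes one, then has the game instance set up and save, printing debug messages along the way.
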(event Custom|LoadGame
  ;[1 1 1] Game Save In Game Base
  (bind _returnvalue (SaveGame|LoadGamefromSlot "1"))
  (Utilities|IsValid _returnvalue
    (:Is%20Valid
      ;;[1 1 1] Load Save Game
      (bind _asbp_game_save (Utilities|Casting|CastToBP_GameSave _returnvalue)
        (:then
          (bind _output_get (Variables|Default|SetAs%20BP%20Game%20Save _asbp_game_save))
          (bind _asgi_base (Utilities|Casting|CastToGI_Base (Game|GetGameInstance)) ; Setting Game Instance for levels
            (:then
              (Utilities|IsValid _asgi_base
                (:Is%20Valid
                  (Default|LoadGame _asgi_base _output_get)
                  (Development|PrintString "Save Loaded"))
                (:Is%20Not%20Valid
                  (Development|PrintString "Game Instance NOT Valid"))))
            (:CastFailed
              (Development|PrintString "Failed cast to GI"))))
        (:CastFailed
          (Development|PrintString "Failed cast to GameSave"))))
    (:Is%20Not%20Valid
      ;;[1 1 1] Create Game Save
      (bind _returnvalue_2 (SaveGame|CreateSaveGameObject "/Game/_GameManager/BP_GameSave.BP_GameSave_C"))
      (bind _output_get_2 (Variables|Default|SetAs%20BP%20Game%20Save _returnvalue_2))
      (SaveGame|SaveGametoSlot _output_get_2 "1")
      (bind _asgi_base_2 (Utilities|Casting|CastToGI_Base (Game|GetGameInstance)) ; Setting Game Instance for levels
        (:then
          (Default|SetupSave _asgi_base_2)
          (Default|SaveGame _asgi_base_2)
          (Development|PrintString "Sace Created / Game Saved"))
        (:CastFailed
          (Development|PrintString "Failed cast to GI"))))))

(event EventBeginPlay
  ;[1 1 1] Game Save In Game Base
  (bind _returnvalue (SaveGame|LoadGamefromSlot "1"))
  (Utilities|IsValid _returnvalue
    (:Is%20Valid
      ;;[1 1 1] Load Save Game
      (bind _asbp_game_save (Utilities|Casting|CastToBP_GameSave _returnvalue)
        (:then
          (bind _output_get (Variables|Default|SetAs%20BP%20Game%20Save _asbp_game_save))
          (bind _asgi_base (Utilities|Casting|CastToGI_Base (Game|GetGameInstance)) ; Setting Game Instance for levels
            (:then
              (Utilities|IsValid _asgi_base
                (:Is%20Valid
                  (Default|LoadGame _asgi_base _output_get)
                  (Development|PrintString "Save Loaded"))
                (:Is%20Not%20Valid
                  (Development|PrintString "Game Instance NOT Valid"))))
            (:CastFailed
              (Development|PrintString "Failed cast to GI"))))
        (:CastFailed
          (Development|PrintString "Failed cast to GameSave"))))
    (:Is%20Not%20Valid
      ;;[1 1 1] Create Game Save
      (bind _returnvalue_2 (SaveGame|CreateSaveGameObject "/Game/_GameManager/BP_GameSave.BP_GameSave_C"))
      (bind _output_get_2 (Variables|Default|SetAs%20BP%20Game%20Save _returnvalue_2))
      (SaveGame|SaveGametoSlot _output_get_2 "1")
      (bind _asgi_base_2 (Utilities|Casting|CastToGI_Base (Game|GetGameInstance)) ; Setting Game Instance for levels
        (:then
          (Default|SetupSave _asgi_base_2)
          (Default|SaveGame _asgi_base_2)
          (Development|PrintString "Sace Created / Game Saved"))
        (:CastFailed
          (Development|PrintString "Failed cast to GI"))))))

(fn ConstructionScript)